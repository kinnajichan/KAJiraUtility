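; BP_JIRATaskActor represents a Jira task as an actor, with events to sync it, comment, change status, upload files or viewport captures, and open it in a browser.
; Each Jira operation constructs an EUB proxy object, initializes it with the actor and delegates the work.
; EUBCOMPJiraSubsystemWidget handles browser opening by TaskID and the widget display, which the Construction Script refreshes through UpdateText.
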(event EventUpdateJiraTask
  ;[0 1 1] JiraTaskを同期し更新する
  (bind _returnvalue (Game|ConstructObjectfromClass "/KAJiraUtility/KAJiraUtility/BP/EUB_JiraTaskUpdateProxy.EUB_JiraTaskUpdateProxy_C"))
  (Class|KAJiraTaskProxyBase|InitTask _returnvalue (Utilities|ResolveSoftReference self))
  (Default|UpdateJiraTask _returnvalue false))

(event EventUpdateText
  ;[0 1 1] テキストの見た目を更新する
  (Default|UpdateWidget (Variables|Default|GetEUB_COMP_JiraSubsystemWidget) (Utilities|ResolveSoftReference self)))

(event EventOpenWebBrowser
  ;[0 1 1] ブラウザでタスクを開く
  (Default|OpenJiraTaskforWebBrowser (Variables|Default|GetEUB_COMP_JiraSubsystemWidget) (Variables|Default|GetTaskID)))

(event EventAddComment
  ;[0 1 1] コメントを追加する
  (bind _returnvalue (Game|ConstructObjectfromClass "/KAJiraUtility/KAJiraUtility/BP/EUB_JiraTaskAddCommentProxy.EUB_JiraTaskAddCommentProxy_C"))
  (Class|KAJiraTaskProxyBase|InitTask _returnvalue (Utilities|ResolveSoftReference self))
  (Default|AddComment _returnvalue))

(event EventChangeStatus
  ;[0 1 1] ステータスを変更する
  (bind _returnvalue (Game|ConstructObjectfromClass "/KAJiraUtility/KAJiraUtility/BP/EUB_JiraTaskChangeStatusProxy.EUB_JiraTaskChangeStatusProxy_C"))
  (Class|KAJiraTaskProxyBase|InitTask _returnvalue (Utilities|ResolveSoftReference self))
  (Default|ChangeStatus _returnvalue))

(event EventUploadCurrentViewportCapture
  ;[0 1 1] 現在のビューポートをキャプチャーしてタスクに添付としてアップロードする
  (bind _returnvalue (Game|ConstructObjectfromClass "/KAJiraUtility/KAJiraUtility/BP/EUB_JiraTaskUploadFileProxy.EUB_JiraTaskUploadFileProxy_C"))
  (Class|KAJiraTaskProxyBase|InitTask _returnvalue (Utilities|ResolveSoftReference self))
  (Default|UploadCurrentViewportCapture _returnvalue))

(event EventUploadFile
  ;[0 1 1] 任意のファイルをタスクに添付としてアップロードする
  (bind _returnvalue (Game|ConstructObjectfromClass "/KAJiraUtility/KAJiraUtility/BP/EUB_JiraTaskUploadFileProxy.EUB_JiraTaskUploadFileProxy_C"))
  (Class|KAJiraTaskProxyBase|InitTask _returnvalue (Utilities|ResolveSoftReference self))
  (Default|UploadSelectedFile _returnvalue))

(fn ConstructionScript
  ;[0 1 1] WidgetComponentの見た目を更新する
  (Class|KAJiraTaskActor|UpdateText))